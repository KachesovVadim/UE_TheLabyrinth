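; GuestDeadZone is an invisible trigger actor that ends the game when the player enters it while a guest is on the level.
; It hides itself at BeginPlay and reacts only to overlaps with player 0's BP_ThirdPersonCharacter.
; On a valid overlap it plays a pistol shot sound and calls FinishGame on the character, choosing one of two ending enum values based on whether the player has a weapon.
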(event EventBeginPlay
  (Rendering|SetActorHiddenInGame true))

(event Collision|EventActorBeginOverlap
  (params (OtherActor :type Actor%20Object%20Reference))
  (bind _returnvalue (Game|GetPlayerCharacter 0))
  (bind _asbp_third_person_character (Utilities|Casting|CastToBP_ThirdPersonCharacter _returnvalue))
  (if (== OtherActor _asbp_third_person_character)
    (if (Default|GetGuestonLevel _asbp_third_person_character)
      (Audio|PlaySound2D "/Game/Sounds/PistolShot.PistolShot" 1.0 1.0 0.0 0 0)
      (if (Variables|/Game/ThirdPerson/Blueprints/BP_ThirdPersonCharacter.BP_ThirdPersonCharacter_C|GetHaveWeapon _asbp_third_person_character)
        (Default|FinishGame _asbp_third_person_character "NewEnumerator3")
        (else
          (Default|FinishGame _asbp_third_person_character "NewEnumerator1"))))))

(fn ConstructionScript)